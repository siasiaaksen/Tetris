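; BP_CheckLine is a line checker for a falling-block puzzle that detects full rows of BP_SingleBlock actors.
; CheckLines loops over the actor's Box components and counts the blocks overlapping each.
; A box with exactly ten blocks adds a fixed step to DropAmount, but nothing here clears or moves blocks.
; The event graph is empty, so CheckLines is never called from within this Blueprint.
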(fn `CheckLines`
  (locals (OverlappingActors :type "Array of Actor Object Reference") (DropAmount :type "Float (double-precision)"))
  (for _array_element (`self.K2_GetComponentsByClass` "/Script/Engine.BoxComponent")
    (set `local.OverlappingActors` (`PrimitiveComponent.GetOverlappingActors` _array_element "/Game/BP/BP_SingleBlock.BP_SingleBlock_C"))
    (if (== (`KismetArrayLibrary.Array_Length` (`local.OverlappingActors`)) 10)
      (set `local.DropAmount` (+ (`local.DropAmount`) 50.0)))))

(fn `UserConstructionScript`)