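; Left side bar actor that sizes and positions itself once when play begins.
; It sets its Z scale from GetYValue, keeping X and Y, and prints that value to screen.
; It then feeds GetXValue through Calculate with IsMinus off to set the root's world Y location, keeping X and Z.
; Overlap, Tick and the construction script are empty.
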(event `self.ReceiveBeginPlay`
  (bind (_returnvalue_x _returnvalue_y _returnvalue_z) (`KismetMathLibrary.BreakVector` (`SceneComponent.K2_GetComponentLocation` (`self.DefaultSceneRoot`))))
  (bind (_returnvalue_x_2 _returnvalue_y_2) (`KismetMathLibrary.BreakVector` (`SceneComponent.K2_GetComponentScale` (`self.DefaultSceneRoot`))))
  (`|ExecutionSequence`
    (:`then_0`
      (bind _returnvalue (`TetrisGameInstance.GetYValue`))
      (`self.SetActorScale3D` (`KismetMathLibrary.MakeVector` _returnvalue_x_2 _returnvalue_y_2 (`KismetMathLibrary.Conv_IntToDouble` _returnvalue)))
      (`KismetSystemLibrary.PrintString` (`KismetStringLibrary.Conv_IntToString` _returnvalue)))
    (:`then_1`
      (bind _returnvalue_2 (`TetrisGameInstance.GetXValue`))
      (bind _returnvalue_3 (`self.Calculate` _returnvalue_2))
      (`SceneComponent.K2_SetWorldLocation` (`self.DefaultSceneRoot`) (`KismetMathLibrary.MakeVector` _returnvalue_x (`KismetMathLibrary.Conv_IntToDouble` _returnvalue_3) _returnvalue_z) false false))))

(event `self.ReceiveTick`
  (params (DeltaSeconds :type "Float (single-precision)")))

(fn `UserConstructionScript`)